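; BP_LobbyPC is the lobby player controller, handling each player's name, ready status and lobby UI.
; On BeginPlay the local controller creates WB_LobbyUI, enables mouse input and submits the name stored in BP_OurGameInstance.
; Name changes and R-key ready toggles update PlayerLobbyInfoPC and pass the controller to BP_LobbyGM, with a delayed retry event available.
; Match start shows a loading screen and disables input.
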(event `self.ReceiveBeginPlay`
  (`self.SetUp`))

(event `TryAgainUpdatingLobbyInfo`
  (`KismetSystemLibrary.Delay` 0.1)
  (bind _asbp_lobby_gm (cast `/Game/Lobby/BP_LobbyGM` (`GameplayStatics.GetGameMode`)))
  (`/Game/Lobby/BP_LobbyGM.UpdatePlayerLobbyInfo` _asbp_lobby_gm self))

(event `SetPlayerNameOnServer`
  (params (`Player Name` :type Text))
  ;[1 1 1] 서버에서 설정한 이름을 로비로 불러오는거
  (setmembers `/Game/Lobby/S_PlayerLobbyInfo` :`StructRef` (`self.PlayerLobbyInfoPC`) :`PlayerName` `Player Name`)
  (bind _asbp_lobby_gm (cast `/Game/Lobby/BP_LobbyGM` (`GameplayStatics.GetGameMode`)))
  (`/Game/Lobby/BP_LobbyGM.UpdatePlayerLobbyInfo` _asbp_lobby_gm self))

(event `ToggleReadyStatusOmServer`
  (bind _playerlobbyinfopc (`self.PlayerLobbyInfoPC`))
  ;[1 1 1] READY Status 설정
  (setmembers `/Game/Lobby/S_PlayerLobbyInfo` :`StructRef` _playerlobbyinfopc :`bReady` (not (`.bReady_8_7C4201DA44C8039D85E383B324098EF9` (break `/Game/Lobby/S_PlayerLobbyInfo` _playerlobbyinfopc))))
  (bind _asbp_lobby_gm (cast `/Game/Lobby/BP_LobbyGM` (`GameplayStatics.GetGameMode`)))
  (`/Game/Lobby/BP_LobbyGM.UpdatePlayerLobbyInfo` _asbp_lobby_gm self))

(event `Key|R`
  (params (Key :type "Key Structure"))
  ;[1 1 1] R누르면 레디 밖힘
  (:`Pressed`
    (`self.ToggleReadyStatusOmServer`)))

(event `OnStrartMatch`
  ;[1 1 1] 스타트메치
  (`/Game/Lobby/WB_LobbyUI.ShowLoadingScreen` (`self.LobbyUI_Ref`))
  (`self.DisableInput` self))

(fn `SetUp`
  ;[1 1 1] UI에 정보 가지고오는거
  (if (`self.IsLocalPlayerController`)
    (set `self.bShowMouseCursor` true)
    (`WidgetBlueprintLibrary.SetInputMode_GameAndUIEx` self null "DoNotLock" false)
    (bind _returnvalue (`|CreateWidget` "/Game/Lobby/WB_LobbyUI.WB_LobbyUI_C"))
    (bind _output_get (set `self.LobbyUI_Ref` _returnvalue))
    (`UserWidget.AddToViewport` _output_get 0)
    (`self.SetPlayerNameOnServer` (`/Game/BluePrint/BP_OurGameInstance.PlayerName` (cast `/Game/BluePrint/BP_OurGameInstance` (`GameplayStatics.GetGameInstance`) :!pure true)))))

(fn `UserConstructionScript`)